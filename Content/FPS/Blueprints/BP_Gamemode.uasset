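; FPS game mode that shows the game menu widget and runs a countdown timer on it.
; BeginPlay prints a start string, adds WBP_GameMenu to the viewport, sets game-only input with a hidden cursor and displays the initial GameTimer.
; Tick calls the Update Timer macro, whose one-second Delay throttles it to decrement GameTimer and refresh the widget once per second.
; Nothing stops the countdown at zero, and the widget removal node is unconnected.
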(event EventBeginPlay
  (bind _returnvalue (Game|GetPlayerController 0))
  (Development|PrintString (Variables|Default|GetStartingStirng) true true "(R=1.000000,G=0.139691,B=0.014063,A=1.000000)" 5.0)
  (bind _returnvalue_2 (UserInterface|CreateWidget "/Game/FPS/Blueprints/GUI/GameMenu/WBP_GameMenu.WBP_GameMenu_C"))
  (bind _output_get (Variables|Default|SetMenu%20Ref _returnvalue_2))
  ;[0.15 0.15 0.15 0.5] adds to screen
  (UserInterface|Viewport|AddtoViewport _output_get 0)
  (Input|SetInputModeGameOnly _returnvalue false)
  (Variables|/Script/Engine.PlayerController|SetbShowMouseCursor _returnvalue false)
  (Default|SetTimer (Variables|Default|GetMenu%20Ref) (Variables|Default|GetGameTimer)))

(event EventTick
  (params (DeltaSeconds :type Float%20%28single-precision%29))
  (Utilities|UpdateTimer))

(fn ConstructionScript)