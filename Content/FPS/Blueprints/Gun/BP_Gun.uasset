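; BP_Gun is a gun actor Blueprint in the FPS folder that provides a basic skeleton for weapons.
; Its OnShoot event forwards start and end positions to a Shooting function, which is a stub that only prints a debug string.
; Getter functions expose the damage, fire rate and maximum bullet distance variables, and the construction script is empty.
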(event EventBeginPlay)

(event Collision|EventActorBeginOverlap
  (params (OtherActor :type Actor%20Object%20Reference)))

(event EventTick
  (params (DeltaSeconds :type Float%20%28single-precision%29)))

(event EventOnShoot
  (params (StartPos :type Vector :default "0, 0, 0") (EndPos :type Vector :default "0, 0, 0"))
  (CallFunction|Shooting StartPos EndPos))

(fn ConstructionScript)

(fn Shooting
  (params (StartPos :type Vector) (EndPos :type Vector))
  (Development|PrintString "BP_Shooting Called"))

(fn GetDamage
  (return (Variables|GunData|GetDamage)))

(fn GetFireRate
  (return (Variables|GunData|GetFireRate)))

(fn GetMaxBulletDistance
  (return (Variables|GunData|GetMaxBulletDistance)))