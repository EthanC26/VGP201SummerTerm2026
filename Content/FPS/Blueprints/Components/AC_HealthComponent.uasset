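; Actor component that tracks health for actors in the FPS game, initialised from its own health, minimum and maximum values on BeginPlay.
; All changes route through SetHealth, which clamps to that range.
; Heal, HealFull and Damage accept only positive amounts, printing a message otherwise.
; It exposes normalized health and an IsDead check at the minimum, but fires no events on change or death.
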(event EventBeginPlay
  (CallFunction|Init (Variables|Default|GetHealth) (Variables|Default|GetMinHealth) (Variables|Default|GetMaxHealth)))

(event EventTick
  (params (DeltaSeconds :type Float%20%28single-precision%29)))

(fn Init
  (params (NewHealth :type Float%20%28double-precision%29) (NewMinHealth :type Float%20%28double-precision%29) (NewMaxHealth :type Float%20%28double-precision%29))
  (Variables|Default|SetMinHealth NewMinHealth)
  (Variables|Default|SetMaxHealth NewMaxHealth)
  (CallFunction|SetHealth NewHealth))

(fn GetHealth
  (return (Variables|Default|GetHealth)))

(fn SetHealth
  (params (NewHealth :type Float%20%28double-precision%29))
  (bind _output_get (Variables|Default|SetHealth (CallFunction|ClampHealth NewHealth)))
  (return _output_get))

(fn ClampHealth
  (params (Value :type Float%20%28double-precision%29))
  (return (Math|Float|Clamp(Float) Value (Variables|Default|GetMinHealth) (Variables|Default|GetMaxHealth))))

(fn GetNormalizedHealth
  (return (Math|Float|Clamp(Float) (/ (CallFunction|GetHealth) (Variables|Default|GetMaxHealth)))))

(fn Heal
  (params (Heal%20Amt :type Float%20%28double-precision%29))
  (if (> Heal%20Amt 0.0)
    (CallFunction|SetHealth (+ (CallFunction|GetHealth) Heal%20Amt))
    (else
      (Development|PrintString "Heal Value must be Positive Bitch"))))

(fn HealFull
  (CallFunction|Heal (Variables|Default|GetMaxHealth)))

(fn Damage
  (params (Damage%20Amt :type Float%20%28double-precision%29))
  (if (> Damage%20Amt 0.0)
    (CallFunction|SetHealth (- (CallFunction|GetHealth) Damage%20Amt))
    (else
      (Development|PrintString "Damage Value muist be postive Bitch"))))

(fn IsDead
  (return (<= (CallFunction|GetHealth) (Variables|Default|GetMinHealth))))